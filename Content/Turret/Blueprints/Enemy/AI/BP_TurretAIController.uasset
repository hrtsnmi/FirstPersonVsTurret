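; AI controller for the turret enemy that runs its behavior tree and tracks perceived targets.
; On BeginPlay it starts the turret behavior tree.
; AI perception updates that pass a cast on the target write it to the enemy Blackboard key when sensed, and clear that key when sensing fails.
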(event OnTargetPerceptionInfoUpdated(AIPerception)
  (params (UpdateInfo :type Actor%20Perception%20Update%20Info%20Structure%20%28by%20ref%29))
  (bind (_targetid _target _stimulus) (Utilities|Struct|BreakActorPerceptionUpdateInfo UpdateInfo))
  (Utilities|Casting|CastTo _target)
  (if (.bsuccessfullysensed _stimulus)
    (AI|Components|Blackboard|SetValueasObject (Variables|Default|GetBlackboard) (Variables|Default|GetEnemyKey) _target)
    (else
      (AI|Components|Blackboard|ClearValue (Variables|Default|GetBlackboard) (Variables|Default|GetEnemyKey)))))

(event EventBeginPlay
  (AI|RunBehaviorTree "/Game/Turret/Blueprints/Enemy/AI/BP_BTTurret.BP_BTTurret"))

(event EventTick
  (params (DeltaSeconds :type Float%20%28single-precision%29)))

(fn ConstructionScript)